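; Wave manager that runs enemy waves defined by a DT_WaveInfo row, announcing progress with on-screen print messages.
; On BeginPlay it caches BP_WaveSpawnPoints actors, waits for the LevelStarted flag, counts down, then spawns enemies at random points and yaw.
; Delay loops poll the flag and stored enemy references; once none are valid, it sets LevelEnded and either awaits the next LevelStarted or announces the final wave complete.
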(event Custom|Display%20Message
  (params (InString :type String))
  (Development|PrintString InString true true "(R=0.000000,G=0.660000,B=1.000000,A=1.000000)" 1e+01))

(event Custom|Final%20Wave%20Finished
  ;[1 1 1] Finished final wave
  (CallFunction|DisplayMessage "FInal wave complete!"))

(event Custom|Spawn%20Next%20Wave
  ;[1 1 1] Increment wave and display message
  (Math|Integer|IncrementInt (Variables|Default|GetcurrentWaveNumber)
    (:%20%20
      (CallFunction|DisplayMessage (Utilities|String|Append "Wave" (Utilities|String|ToString(Integer) (Variables|Default|GetcurrentWaveNumber)) "begin!"))
      ;[1 1 1] Spawn enemies and check if valid
      (CallFunction|SpawnEnemiesforCurrentWave) ; Spawns the eniemes for the waves
      (bind _benemiesdefeated (CallFunction|CheckifEnemiesAreDefeated :!label _label)) ; Checks if enemies are defeated
      (if _benemiesdefeated
        (Variables|WaveSettings|SetbLevelEnded true) ; Sets level ended to true
        ;[1 1 1] Wave finished feedback
        (CallFunction|DisplayMessage "Wave complete!")
        (Utilities|FlowControl|Delay 0.2)
        ;[1 1 1] Check if final wave
        (bind (_lastindex _currentwavenumber) (CallFunction|GetLastIndexOfWaveInfo))
        (if (== _lastindex _currentwavenumber)
          ;[1 1 1] Finish/Start next wave
          (CallFunction|FinalWaveFinished)
          (else
            ;[1 1 1] Checks to see if the level has started
            (Utilities|CheckifLevelHasStarted)
            (CallFunction|SpawnNextWave)
            (Variables|WaveSettings|SetbLevelEnded false) ; Setsl to false when a new level starts
          ))
        (else
          (Utilities|FlowControl|Delay 1.0)
          (goto _label))))))

(event EventBeginPlay
  ;[0.1481 1 0.8297] Begin play
  ;;[1 0.1458 0.1458] Initialize important variables
  (CallFunction|Init)
  ;;[1 1 1] Checks to see if the level has started
  (Utilities|CheckifLevelHasStarted)
  ;;[1 1 1] Countdown until start
  (Utilities|CountdownUntilStart)
  ;;[1 0.1042 0.1042] Spawns the next wave
  (CallFunction|SpawnNextWave))

(fn ConstructionScript)

(fn Init
  ;[1 1 1] Data Table
  (bind _returnvalue (Utilities|GetDataTableRow "/Game/ProjectNinja/Core/WaveManager/DT_WaveInfo.DT_WaveInfo" (Variables|Default|GetwaveSettingsRowName))
    (:then
      (Variables|Default|SetwaveSettings _returnvalue)
      ;[1 1 1] Counter
      (Variables|WaveSettings|SetCounter (Variables|Default|GetInitialCountdown))
      ;[1 1 1] Save Spawn Points
      (bind _outactors (Actor|GetAllActorsOfClass "/Game/ProjectNinja/Placeables/BP_WaveSpawnPoints.BP_WaveSpawnPoints_C"))
      (Variables|Default|SetspawnPointReferences _outactors))))

(fn SpawnEnemiesforCurrentWave
  (bind _wavesettings (Variables|Default|GetwaveSettings))
  (bind _currentwavenumber (Variables|Default|GetcurrentWaveNumber))
  (bind _output (Utilities|Array|Get(acopy) (.waveinfo _wavesettings) _currentwavenumber))
  (bind (_enemyclasses _classamount) (Utilities|Struct|BreakS_WaveEnemyInfo _output))
  (for _array_element _enemyclasses
    (for _index (range 1 (Utilities|Array|Get(acopy) _classamount))
      (bind _returnvalue (Game|SpawnActorfromClass _array_element (CallFunction|GetRandomSpawnPoint) "Undefined" 0 0))
      (Utilities|Array|Add (Variables|Default|GetcurrentEnemyReferences) _returnvalue))
    (return)))

(fn GetRandomSpawnPoint
  (return (Math|Transform|MakeTransform (Transformation|GetWorldLocation (Variables|/Game/ProjectNinja/Placeables/BP_WaveSpawnPoints.BP_WaveSpawnPoints_C|GetspawnPointTransform (.OutItem (Utilities|Array|Random (Variables|Default|GetspawnPointReferences))))) (Math|Rotator|MakeRotator 0.0 0.0 (Math|Random|RandomFloatinRange 0.0 3.6e+02)))))

(fn CheckifEnemiesAreDefeated
  (for _array_element (Variables|Default|GetcurrentEnemyReferences) ; Checks all the enemies in the stored reference
    (Utilities|IsValid _array_element
      (:Is%20Valid
        (return false))))
  (return true) ; Returns true if the enemies are defeated
)

(fn GetLastIndexOfWaveInfo
  (return (Utilities|Array|LastIndex (Utilities|Struct|BreakS_WaveInfo (Variables|Default|GetwaveSettings))) (Variables|Default|GetcurrentWaveNumber)))