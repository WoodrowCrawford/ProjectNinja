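; BP_Player is the player character, handling axis-driven movement, mouse-style look and jumping.
; MoveX and MoveY add movement along the actor's right and forward vectors, while LookX and LookY feed controller yaw and pitch.
; A TestBoxKiller overlap component destroys any BP_TestCube it begins overlapping, which appears to be test logic.
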(event OnComponentBeginOverlap(TestBoxKiller)
  (params (OverlappedComponent :type Primitive%20Component%20Object%20Reference) (OtherActor :type Actor%20Object%20Reference) (OtherComp :type Primitive%20Component%20Object%20Reference) (OtherBodyIndex :type Integer) (bFromSweep :type Boolean) (SweepResult :type Hit%20Result%20Structure%20%28by%20ref%29))
  (bind _asbp_test_cube (Utilities|Casting|CastToBP_TestCube OtherActor))
  (Actor|DestroyActor _asbp_test_cube))

(event Input|ActionEvents|InputActionJump
  (params (Key :type Key%20Structure :default "None"))
  ;[1 1 1] Jump Action
  (:Pressed
    (Character|Jump)))

(event Input|AxisEvents|InputAxisMoveX
  (params (AxisValue :type Float%20%28single-precision%29))
  ;[1 1 1] Move Left/Right
  (Pawn|Input|AddMovementInput (Transformation|GetActorRightVector) AxisValue false))

(event Input|AxisEvents|InputAxisMoveY
  (params (AxisValue :type Float%20%28single-precision%29))
  ;[1 1 1] Move Up/Down
  (Pawn|Input|AddMovementInput (Transformation|GetActorForwardVector) AxisValue false))

(event Input|AxisEvents|InputAxisLookX
  (params (AxisValue :type Float%20%28single-precision%29))
  ;[1 1 1] Look Function
  (Pawn|Input|AddControllerYawInput AxisValue))

(event Input|AxisEvents|InputAxisLookY
  (params (AxisValue :type Float%20%28single-precision%29))
  ;[1 1 1] Look Function
  (Pawn|Input|AddControllerPitchInput AxisValue))

(fn ConstructionScript)