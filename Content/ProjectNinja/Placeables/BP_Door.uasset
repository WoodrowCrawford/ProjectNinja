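; BP_Door is a placeable door that signals a level start to the wave manager when the player enters its trigger.
; On overlap it pulses the manager's LevelStarted flag true for one second, then resets it and calls SetDoorInactive.
; That function hides the door, removes its collision and disables trigger overlap events.
; If the flag is already set, the overlap only prints a debug message.
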(event OnComponentBeginOverlap(DoorTrigger)
  (params (OverlappedComponent :type Primitive%20Component%20Object%20Reference) (OtherActor :type Actor%20Object%20Reference) (OtherComp :type Primitive%20Component%20Object%20Reference) (OtherBodyIndex :type Integer) (bFromSweep :type Boolean) (SweepResult :type Hit%20Result%20Structure%20%28by%20ref%29))
  (Utilities|Casting|CastToBP_Player OtherActor)
  ;[1 1 1] Checks to see if level is started
  (if (Variables|/Game/ProjectNinja/Core/WaveManager/BP_WaveManager.BP_WaveManager_C|GetbLevelStarted (Variables|Default|GetWaveManagerReference))
    ;[0.1816 0.1744 1] Debug
    (Development|PrintString "Level is already started")
    (else
      ;[1 1 1] Starts the level, then sets the bool to be false
      (Variables|/Game/ProjectNinja/Core/WaveManager/BP_WaveManager.BP_WaveManager_C|SetbLevelStarted (Variables|Default|GetWaveManagerReference) true)
      (Utilities|FlowControl|Delay 1.0)
      (Variables|/Game/ProjectNinja/Core/WaveManager/BP_WaveManager.BP_WaveManager_C|SetbLevelStarted (Variables|Default|GetWaveManagerReference) false)
      ;[1 1 1] Sets the door/trigger to be inactive
      (CallFunction|SetDoorInactive) ; Sets the door to be inactive
    )))

(fn ConstructionScript)

(fn SetDoorInactive
  (bind _door (Variables|Default|GetDoor))
  (Collision|SetCollisionEnabled _door "NoCollision")
  (Development|SetHiddeninGame _door true false)
  (Variables|/Script/Engine.PrimitiveComponent|SetbGenerateOverlapEvents (Variables|Default|GetDoorTrigger) false))